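; BP_Cube is a physics cube whose motion can be rewound through time, toggled by the Rewind and Forward events.
; While moving forward, Tick appends the mesh's world transform and physics velocities to unbounded history arrays.
; While rewinding, it pops and applies entries newest first, holding the oldest transform once history runs out.
; Linear and angular velocity share one Transform entry, packed into its Location and Scale fields.
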(event `/Game/Blueprints/BPI_TimeControl.Rewind`
  (set `self.Rewinding` true))

(event `/Game/Blueprints/BPI_TimeControl.Forward`
  (set `self.Rewinding` false))

(event `self.ReceiveTick`
  (params (DeltaSeconds :type "Float (single-precision)"))
  (bind _mesh (`self.Mesh`))
  (bind _mesh_2 (`self.Mesh`))
  (bind _actorvelocity (`self.ActorVelocity`))
  (bind _actortransform (`self.Actortransform`))
  (bind _actortransform_2 (`self.Actortransform`))
  (`|ExecutionSequence`
    (:`then_0`
      (if (`self.Rewinding`)
        (if (> (`KismetArrayLibrary.Array_LastIndex` (`self.Actortransform`)) 0)
          (`SceneComponent.K2_SetWorldTransform` (`self.Mesh`) (`|GetArrayItem` _actortransform_2 (`KismetArrayLibrary.Array_LastIndex` _actortransform_2)) false false)
          (if (> (`KismetArrayLibrary.Array_LastIndex` (`self.Actortransform`)) 0)
            (`KismetArrayLibrary.Array_Remove` (`self.Actortransform`) (`KismetArrayLibrary.Array_LastIndex` (`self.Actortransform`))))
          (else
            (`SceneComponent.K2_SetWorldTransform` (`self.Mesh`) (`|GetArrayItem` _actortransform (`KismetArrayLibrary.Array_LastIndex` _actortransform)) false false)))
        (else
          (`KismetArrayLibrary.Array_Add` (`self.Actortransform`) (`SceneComponent.K2_GetComponentToWorld` (`self.Mesh`))))))
    (:`then_1`
      (if (`self.Rewinding`)
        (if (> (`KismetArrayLibrary.Array_LastIndex` (`self.ActorVelocity`)) 0)
          (`PrimitiveComponent.SetPhysicsLinearVelocity` _mesh_2 (.location (`|GetArrayItem` _actorvelocity (`KismetArrayLibrary.Array_LastIndex` _actorvelocity))) false "None")
          (`PrimitiveComponent.SetPhysicsAngularVelocityInDegrees` _mesh_2 (.scale (`|GetArrayItem` _actorvelocity (`KismetArrayLibrary.Array_LastIndex` _actorvelocity))) false "None")
          (if (> (`KismetArrayLibrary.Array_LastIndex` (`self.ActorVelocity`)) 0)
            (`KismetArrayLibrary.Array_Remove` (`self.ActorVelocity`) (`KismetArrayLibrary.Array_LastIndex` (`self.ActorVelocity`)))))
        (else
          (bind _returnvalue (`PrimitiveComponent.GetPhysicsLinearVelocity` _mesh "None"))
          (`KismetArrayLibrary.Array_Add` (`self.ActorVelocity`) (`KismetMathLibrary.MakeTransform` _returnvalue (struct) (`PrimitiveComponent.GetPhysicsAngularVelocityInDegrees` _mesh "None"))))))))

(fn `UserConstructionScript`)